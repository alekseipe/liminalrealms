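; BP_CardAttackEffect is a card effect actor that sends a colored Niagara absorption particle effect toward a destination position.
; BeginPlay picks the Niagara system by EffectType, such as Trap, Sword, Shield, Fire, Lightning or Heart.
; Tick moves the effect component toward DestinationPosition at constant speed with VInterpToConstant.
; On arrival, a DoOnce deactivates the effect after a short delay, then destroys the actor once a further delay passes.
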(event EventTick
  (params (DeltaSeconds :type Float%20%28single-precision%29))
  (bind _main (Variables|Default|GetMain))
  (bind _destinationposition (Variables|Default|GetDestinationPosition))
  (bind _returnvalue (Transformation|GetWorldLocation _main))
  (bind _returnvalue_2 (Math|Interpolation|VInterptoConstant _returnvalue _destinationposition DeltaSeconds 2e+02))
  (Transformation|SetWorldLocation _main _returnvalue_2 false false)
  (if (< (Math|Vector|Distance(Vector) _returnvalue_2 _destinationposition) 1.0)
    (Utilities|FlowControl|DoOnce false
      (:Completed
        (Utilities|FlowControl|Delay 0.2)
        (Components|Activation|SetActive (Variables|Default|GetMain) false false)
        (Utilities|FlowControl|Delay 1.0)
        (Actor|DestroyActor)))))

(event EventBeginPlay
  (Class|NiagaraComponent|SetAsset (Variables|Default|GetMain) (Utilities|Select :Index (Variables|Default|GetEffectType) :NewEnumerator8 "/Game/AbsorbtionFX/FX/NS_Absorption_Black.NS_Absorption_Black" :NewEnumerator1 "/Game/AbsorbtionFX/FX/NS_Absorption_Yellow.NS_Absorption_Yellow" :NewEnumerator2 "/Game/AbsorbtionFX/FX/NS_Absorption_Blue.NS_Absorption_Blue" :NewEnumerator7 "/Game/AbsorbtionFX/FX/NS_Absorption_Orange.NS_Absorption_Orange" :NewEnumerator9 "/Game/AbsorbtionFX/FX/NS_Absorption_Teal.NS_Absorption_Teal" :NewEnumerator10 "/Game/AbsorbtionFX/FX/NS_Absorption_Green.NS_Absorption_Green" :NewEnumerator11 0) true))

(fn ConstructionScript)