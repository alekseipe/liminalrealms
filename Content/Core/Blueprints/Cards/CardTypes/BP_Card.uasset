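; BP_Card is a clickable card actor of type Sword, Shield or Fire, owned by a BP_CardGrid.
; On BeginPlay it sets its text label and mesh material from CardData.
; A left click during one specific GM_Main game state adds its index to the grid's combo.
; DoDamage sends type and value to BP_EnemyManager against enemy slot 0, identically for all three types, Shield included.
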(event OnClicked(StaticMesh)
  (params (TouchedComponent :type Primitive%20Component%20Object%20Reference) (ButtonPressed :type Key%20Structure :default "None"))
  (if (== ButtonPressed "LeftMouseButton")
    (bind _asgm_main (Utilities|Casting|CastToGM_Main (Game|GetGameMode)))
    (if (Utilities|Enum|Equal(Enum) (Variables|/Game/Core/Blueprints/GM_Main.GM_Main_C|GetCurrentGameState _asgm_main) "NewEnumerator3")
      (bind _asbp_card_grid (Utilities|Casting|CastToBP_CardGrid (Components|GetOwner)))
      (Default|AddtoCombo _asbp_card_grid (Variables|Default|GetCardIndex)))))

(event EventBeginPlay
  (switch Utilities|FlowControl|Switch|SwitchonE_CardType (.cardtype (Variables|Default|GetCardData))
    (:NewEnumerator1
      (Rendering|Components|TextRender|SetText (Variables|Default|GetCardTXT) (Utilities|Text|FormatText "DMG:{Damage}" (.damage (Variables|Default|GetCardData))))
      (Rendering|Material|SetMaterial (Variables|Default|GetStaticMesh) 0 "/Game/Core/Materials/MAT_Red.MAT_Red"))
    (:NewEnumerator2
      (Rendering|Components|TextRender|SetText (Variables|Default|GetCardTXT) (Utilities|Text|FormatText "BLK:{Block}" (.damage (Variables|Default|GetCardData))))
      (Rendering|Material|SetMaterial (Variables|Default|GetStaticMesh) 0 "/Game/Core/Materials/MAT_Blue.MAT_Blue"))
    (:NewEnumerator7
      (Rendering|Components|TextRender|SetText (Variables|Default|GetCardTXT) (Utilities|Text|FormatText "FIRE:{Fire}" (.damage (Variables|Default|GetCardData))))
      (Rendering|Material|SetMaterial (Variables|Default|GetStaticMesh) 0 "/Engine/MapTemplates/Materials/BasicAsset03.BasicAsset03"))))

(fn ConstructionScript)

(fn DoDamage
  (bind _carddata (Variables|Default|GetCardData))
  (switch Utilities|FlowControl|Switch|SwitchonE_CardType (.cardtype (Variables|Default|GetCardData))
    (:NewEnumerator1
      _)
    (:NewEnumerator2
      _)
    (:NewEnumerator7
      _))
  (bind _returnvalue (Actor|GetActorOfClass "/Game/Core/Blueprints/Enemies/BP_EnemyManager.BP_EnemyManager_C"))
  (Default|DamageEnemy _returnvalue 0 (.cardtype _carddata) (.damage _carddata)))