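; Player character Blueprint that tracks health and shows it on a health bar widget.
; On BeginPlay it binds to the next-level and next-turn events of GM_Main.
; A new level restores health to maximum and pushes it to WUI_PlayerHealthbar through its widget component, ignoring the difficulty value.
; The next-turn handler is empty.
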(event Custom|NextTurn)

(event Custom|NextLevel
  (params (Difficulty :type Float%20%28double-precision%29))
  (Variables|Default|SetHealth (Variables|Default|GetMaxHealth))
  (CallFunction|UpdateHealthBar))

(event EventBeginPlay
  (bind _asgm_main (Utilities|Casting|CastToGM_Main (Game|GetGameMode)))
  (EventDispatchers|BindEventtoNextLevel _asgm_main (delegate Custom|NextLevel))
  (EventDispatchers|BindEventtoNextTurn _asgm_main (delegate Custom|NextTurn)))

(fn ConstructionScript)

(fn UpdateHealthBar
  (bind _aswui_player_healthbar (Utilities|Casting|CastToWUI_PlayerHealthbar (UserInterface|GetWidget (Variables|Default|GetWidget))))
  (Default|SetHealthPercent _aswui_player_healthbar (Variables|Default|GetHealth) (Variables|Default|GetMaxHealth)))