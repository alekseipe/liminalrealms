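; BP_LevelFloor_Stage is a stage floor actor that sets its look to match the current world type when a map starts.
; On BeginPlay it binds MapStart to the GM_Main game mode's map start event.
; MapStart waits one tick, then looks up the game mode's WorldType in the WorldTypeBackground map and applies that material to the first slot of its static mesh.
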(event Custom|MapStart
  (params (bNewGame :type Boolean) (bLoading :type Boolean) (bPlayerWon :type Boolean))
  (Utilities|FlowControl|DelayUntilNextTick)
  (bind _asgm_main (Utilities|Casting|CastToGM_Main (Game|GetGameMode)))
  (Rendering|Material|SetMaterial (Variables|Default|GetStaticMesh) 0 (.Value (Utilities|Map|Find (Variables|Default|GetWorldTypeBackground) (Variables|/Game/Core/Blueprints/GM_Main.GM_Main_C|GetWorldType _asgm_main)))))

(event EventBeginPlay
  (bind _asgm_main (Utilities|Casting|CastToGM_Main (Game|GetGameMode)))
  (EventDispatchers|BindEventtoMapStart _asgm_main (delegate Custom|MapStart)))

(fn ConstructionScript)