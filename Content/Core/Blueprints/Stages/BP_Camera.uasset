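; BP_Camera is a stage camera built to glide between a default framing and an enemy framing, but its movement is currently disconnected.
; TurnEndDamageEnemies sets the destination position and ortho width to the enemy values.
; BeginPlay and Tick are empty, leaving the default setup, GM_Main binding and constant-speed interpolation of location and ortho width, with end snap, as unreachable logic.
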(event Custom|Turn%20End%20Damage%20Enemies
  (Variables|Default|SetDestinationPosition (Variables|Default|GetEnemyPosition))
  (Variables|Default|SetDestinationOrtho (Variables|Default|GetEnemyOrtho)))

(event EventTick
  (params (DeltaSeconds :type Float%20%28single-precision%29)))

(event EventBeginPlay)

(fn ConstructionScript)