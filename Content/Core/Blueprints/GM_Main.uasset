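; Main game mode for a turn-based card game, driving the flow between map, level prep, turns and win/fail screens.
; Each phase sets the game state and notifies listeners through dispatcher-style calls, often staggered by next-tick delays.
; Reward levels play a harder battle before their Shrine or Upgrade; boss wins generate a new map and expand the deck.
; Timelines crossfade music chosen by level type and prep phase, replaying when playback stops.
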(event Custom|TurnEnd
  (Variables|Default|SetCurrentGameState "NewEnumerator2") ; Play TurnEnd
  (Utilities|FlowControl|DelayUntilNextTick)
  (Default|CallNextTurnEnd)
  (Utilities|FlowControl|DelayUntilNextTick)
  (Utilities|FlowControl|Delay 1.5)
  (if (Utilities|Enum|Equal(Enum) (Variables|Default|GetCurrentGameState) "NewEnumerator2") ; Stop if player won by defeating enemies
    (CallFunction|TurnStart false) ; If level not ended, start next turn
  ))

(event Custom|LevelStart
  (params (Difficulty :type Float%20%28double-precision%29) (LevelType :type E_LevelType%20Enum :default "NewEnumerator0") (bIsRewardLevel :type Boolean))
  (Variables|Default|SetCurrentGameState "NewEnumerator0")
  (Variables|Default|SetPostLevelType "NewEnumerator6")
  (Variables|Default|SetDifficulty Difficulty)
  (if bIsRewardLevel ; Play level type as secondary
    (Variables|Default|SetLevelType "NewEnumerator0")
    (Variables|Default|SetPostLevelType LevelType)
    (else
      (Variables|Default|SetLevelType LevelType)))
  (Variables|Default|SetbIsPrepAudio true)
  (CallFunction|PlayNewMusic) ; Play Prep Music
  (Default|CallNextLevelStart (Math|Float|SelectFloat (+ (Variables|Default|GetDifficulty) 1.0) (Variables|Default|GetDifficulty) bIsRewardLevel) (Variables|Default|GetLevelType))
  (switch Utilities|FlowControl|Switch|SwitchonE_LevelType (Variables|Default|GetLevelType)
    (:NewEnumerator1
      _)
    (:NewEnumerator2
      _))
  (CallFunction|LevelPostStart))

(event Custom|LevelEnd
  (params (bPlayerWon :type Boolean))
  (Variables|Default|SetCurrentGameState "NewEnumerator4")
  (Variables|Default|SetbPlayerWon bPlayerWon)
  (Utilities|FlowControl|DelayUntilNextTick)
  (Default|CallNextLevelEnd)
  (Utilities|FlowControl|Delay 1.5)
  (bind _returnvalue (UserInterface|CreateWidget (select (Variables|Default|GetbPlayerWon) "/Game/Core/Blueprints/WUI_LevelWin.WUI_LevelWin_C" "/Game/Core/Blueprints/WUI_LevelFail.WUI_LevelFail_C") (Game|GetPlayerController 0)))
  (bind _output_get (Variables|Default|SetLevelEndWidget _returnvalue))
  (if (not (UserInterface|Viewport|IsinViewport _output_get))
    (UserInterface|Viewport|AddtoViewport _output_get 0)))

(event Custom|LevelPostStart
  (Variables|Default|SetCurrentGameState "NewEnumerator6")
  (Utilities|FlowControl|DelayUntilNextTick)
  (Default|CallNextLevelPostStart (Variables|Default|GetLevelType))
  (Utilities|FlowControl|DelayUntilNextTick)
  (Variables|Default|SetbIsPrepAudio false)
  (CallFunction|PlayNewMusic) ; Play Battle Music
  (CallFunction|TurnStart true))

(event Custom|TurnStart
  (params (bIsFirstTurn :type Boolean))
  (Variables|Default|SetCurrentGameState "NewEnumerator3")
  (Utilities|FlowControl|DelayUntilNextTick)
  (Default|CallNextTurnStart bIsFirstTurn))

(event Custom|PlayNewMusic
  (bind _audio (Variables|Default|GetAudio))
  ;[0.07926 0.3024 1] Music
  (bind _fadein (Timeline|Timeline ReverseFromEnd)
    (:Update
      (Audio|Components|Audio|SetVolumeMultiplier _audio _fadein :!class /Script/Engine.AudioComponent))
    (:Finished
      (Audio|Components|Audio|SetSound _audio (.Value (Utilities|Map|Find (select (Variables|Default|GetbIsPrepAudio) (Variables|Default|GetLevelPrepAudioMap) (Variables|Default|GetLevelAudioMap)) (Variables|Default|GetLevelType))))
      (Audio|Components|Audio|Play _audio 0.0)
      (bind _fadein_2 (Timeline|FadeIn PlayFromStart)
        (:Update
          (Audio|Components|Audio|SetVolumeMultiplier (Variables|Default|GetAudio) _fadein_2 :!class /Script/Engine.AudioComponent))))))

(event Custom|GameQuit
  (CallFunction|CleanupLevelEndWidget)
  (Utilities|FlowControl|DelayUntilNextTick)
  (Game|QuitGame 0 "Quit" false))

(event Custom|GameRestart
  (bind _returnvalue (Game|GetCurrentLevelName true))
  (Game|OpenLevel(byName) (Utilities|String|StringToName _returnvalue)))

(event Custom|NextMapStart
  (params (bGameStart :type Boolean) (bPlayerWon :type Boolean))
  (Variables|Default|SetCurrentGameState "NewEnumerator5")
  (if (not (and bPlayerWon (Utilities|Enum|Equal(Enum) (Variables|Default|GetLevelType) "NewEnumerator4")))
    _
    (else
      (CallFunction|NewMap)))
  (Variables|Default|SetLevelType "NewEnumerator5")
  (CallFunction|CleanupLevelEndWidget)
  (if (Utilities|Enum|NotEqual(Enum) (Variables|Default|GetPostLevelType) "NewEnumerator6") ; If post level set,
    (CallFunction|LevelStart (Variables|Default|GetDifficulty) (Variables|Default|GetPostLevelType) false)
    (else
      (Variables|Default|SetbIsPrepAudio false)
      (CallFunction|PlayNewMusic) ; Play Map Music
    )))

(event EventTick
  (params (DeltaSeconds :type Float%20%28single-precision%29))
  ;[0.07926 0.3024 1] Music
  (if (not (Audio|Components|Audio|IsPlaying (Variables|Default|GetAudio)))
    (Utilities|FlowControl|DoOnce false :!label _label
      (:Completed
        (CallFunction|PlayNewMusic)
        (Utilities|FlowControl|Delay 1.0)
        (goto _label Reset)))))

(event EventBeginPlay
  (Variables|Default|SetCurrentGameState "NewEnumerator5")
  (EventDispatchers|BindEventtoMapStart (delegate Custom|NextMapStart))
  (Utilities|FlowControl|DelayUntilNextTick)
  (Default|CallMapStart true false))

(fn ConstructionScript)

(fn CleanupLevelEndWidget
  (bind _levelendwidget (Variables|Default|GetLevelEndWidget)
    (:then
      (Widget|RemovefromParent _levelendwidget)
      (Variables|Default|SetLevelEndWidget 0))
    (:else)))

(fn NewMap
  (bind _returnvalue (Actor|GetActorOfClass "/Game/Core/Blueprints/GameMap/BP_LevelMap.BP_LevelMap_C")) ; Create new map after boss is defeated
  (Default|CreateMap _returnvalue false)
  (bind _returnvalue_2 (Actor|GetActorOfClass "/Game/Core/Blueprints/Cards/BP_CardGrid.BP_CardGrid_C")) ; Add new card type to inventory
  (bind _baddedcards (Default|AddNewCardTypetoInventory _returnvalue_2))
  (if _baddedcards
    (Default|IncrementDeckSize _returnvalue_2 10)))