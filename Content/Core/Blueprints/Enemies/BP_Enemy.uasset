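; Turn-based enemy actor configured from a data asset that sets its base and shell meshes, materials, animation, health, damage and attack list.
; ProcessTurn counts turns to each attack, which damages the player or adds trap cards to the card grid's deck, with more for bosses.
; The next attack is picked at random and telegraphed on the health bar widget.
; Taking damage briefly swaps in hit materials that copy the original textures.
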(event EventBeginPlay
  (CallFunction|SetupEnemy)
  (CallFunction|UpdateHealthBar))

(event EventTick
  (params (DeltaSeconds :type Float%20%28single-precision%29))
  (if (Variables|Default|GetbTookDamage)
    (Variables|Default|SetbTookDamage false)
    (Utilities|FlowControl|Sequence
      (:then_0
        (Utilities|IsValid (Variables|Default|GetMeshMaterial_Hit)
          (:Is%20Valid
            (Rendering|Material|SetMaterial (Variables|Character|GetMesh) 0 (Variables|Default|GetMeshMaterial_Hit)))))
      (:then_1
        (Utilities|IsValid (Variables|Default|GetShellMaterial_Hit)
          (:Is%20Valid
            (Rendering|Material|SetMaterial (Variables|Default|GetMesh%20Component) 0 (Variables|Default|GetShellMaterial_Hit)))))
      (:then_2
        (Utilities|FlowControl|Delay 0.31)
        (CallFunction|SetMaterialInstances (Variables|Default|GetDataAsset))))))

(fn ConstructionScript
  (CallFunction|SetupEnemy))

(fn SetSkeletalMeshes
  (params (DataAsset :type PDA%20Enemy%20Data%20Object%20Reference))
  (Components|SkeletalMesh|SetSkeletalMeshAsset (Variables|Character|GetMesh) (Variables|/Game/Core/Blueprints/Enemies/PDA_EnemyData.PDA_EnemyData_C|GetBase%20Mesh DataAsset))
  (Components|SkeletalMesh|SetSkeletalMeshAsset (Variables|Default|GetMesh%20Component) (Variables|/Game/Core/Blueprints/Enemies/PDA_EnemyData.PDA_EnemyData_C|GetShell%20Mesh DataAsset))
  (return))

(fn SetMaterialInstances
  (params (DataAsset :type PDA%20Enemy%20Data%20Object%20Reference))
  (bind _returnvalue (Rendering|Material|CreateDynamicMaterialInstance (Variables|/Game/Core/Blueprints/Enemies/PDA_EnemyData.PDA_EnemyData_C|GetBase%20Material%20Instance DataAsset) "None" "None" :!class /Script/Engine.KismetMaterialLibrary))
  (bind _output_get (Variables|Default|SetMeshMaterial _returnvalue))
  (Rendering|Material|SetMaterial (Variables|Character|GetMesh) 0 _output_get)
  (bind _returnvalue_2 (Rendering|Material|CreateDynamicMaterialInstance (Variables|/Game/Core/Blueprints/Enemies/PDA_EnemyData.PDA_EnemyData_C|GetShell%20Material%20Instance DataAsset) "None" "None" :!class /Script/Engine.KismetMaterialLibrary))
  (bind _output_get_2 (Variables|Default|SetShellMaterial _returnvalue_2))
  (Rendering|Material|SetMaterial (Variables|Default|GetMesh%20Component) 0 _output_get_2))

(fn TakeDamage
  (params (Damage :type Float%20%28double-precision%29))
  (LocalVariables|SetLDamage Damage)
  (if (not (Variables|Default|GetbIsDead)) ; If alive
    (LocalVariables|SetLDamageTaken (- (Variables|Default|GetHealth) (Math|Float|Max(Float) (- (Variables|Default|GetHealth) (LocalVariables|GetLDamage)) 0.0))) ; Gets damage taken (considering cutoff for minimum)
    (Variables|Default|SetHealth (Math|Float|Max(Float) (- (Variables|Default|GetHealth) (LocalVariables|GetLDamage)) 0.0))
    (CallFunction|UpdateHealthBar)
    (Variables|Default|SetbTookDamage (> (LocalVariables|GetLDamageTaken) 0.0))
    (Variables|Default|SetbIsDead (<= (Variables|Default|GetHealth) 0.0))))

(fn UpdateHealthBar
  (bind _aswui_enemy_healthbar (Utilities|Casting|CastToWUI_EnemyHealthbar (UserInterface|GetWidget (Variables|Default|GetWidget))))
  (Default|SetHealthPercent _aswui_enemy_healthbar (Variables|Default|GetHealth) (Variables|Default|GetMaxHealth)))

(fn SetupEnemy
  (bind _dataasset (Variables|Default|GetDataAsset)
    (:then
      (Utilities|FlowControl|Sequence
        (:then_0
          (CallFunction|SetSkeletalMeshes _dataasset)
          (CallFunction|SetMaterialInstances _dataasset)
          (Class|SkeletalMeshComponent|SetAnimClass (Variables|Character|GetMesh) (Variables|/Game/Core/Blueprints/Enemies/PDA_EnemyData.PDA_EnemyData_C|GetAnimation%20Blueprint _dataasset))
          (Class|SkeletalMeshComponent|SetAnimClass (Variables|Default|GetMesh%20Component) (Variables|/Game/Core/Blueprints/Enemies/PDA_EnemyData.PDA_EnemyData_C|GetAnimation%20Blueprint _dataasset)))
        (:then_1
          (Utilities|FlowControl|Sequence ; Set hit materials
            (:then_0
              (Utilities|IsValid (Variables|Default|GetMeshMaterial)
                (:Is%20Valid
                  (bind _returnvalue (Rendering|Material|CreateDynamicMaterialInstance "/Game/Core/Blueprints/Enemies/MAT_Damage_Inst.MAT_Damage_Inst" "None" "None" :!class /Script/Engine.KismetMaterialLibrary))
                  (bind _output_get (Variables|Default|SetMeshMaterial_Hit _returnvalue))
                  (CallFunction|SetHitMaterialInstTextures (Variables|Default|GetMeshMaterial) _output_get))))
            (:then_1
              (Utilities|IsValid (Variables|Default|GetShellMaterial)
                (:Is%20Valid
                  (bind _returnvalue_2 (Rendering|Material|CreateDynamicMaterialInstance "/Game/Core/Blueprints/Enemies/MAT_Damage_Inst.MAT_Damage_Inst" "None" "None" :!class /Script/Engine.KismetMaterialLibrary))
                  (bind _output_get_2 (Variables|Default|SetShellMaterial_Hit _returnvalue_2))
                  (CallFunction|SetHitMaterialInstTextures (Variables|Default|GetShellMaterial) _output_get_2))))))
        (:then_2
          (bind _output_get_3 (Variables|Default|SetMaxHealth (Variables|/Game/Core/Blueprints/Enemies/PDA_EnemyData.PDA_EnemyData_C|GetHealth (Variables|Default|GetDataAsset))))
          (Variables|Default|SetHealth _output_get_3)
          (CallFunction|UpdateHealthBar)
          (if (Variables|/Game/Core/Blueprints/Enemies/PDA_EnemyData.PDA_EnemyData_C|GetbIsBoss (Variables|Default|GetDataAsset)) ; If Boss,
            (Transformation|AddLocalOffset (Variables|Default|GetWidget) "-90.000000,30.000000,0.000000" false false) ; Move Bar
          ))
        (:then_3
          (Variables|Default|SetDamage (Variables|/Game/Core/Blueprints/Enemies/PDA_EnemyData.PDA_EnemyData_C|GetDamage (Variables|Default|GetDataAsset))))
        (:then_4
          (Variables|Default|SetAttackEffects (Variables|/Game/Core/Blueprints/Enemies/PDA_EnemyData.PDA_EnemyData_C|GetAttackEffects (Variables|Default|GetDataAsset)))
          (CallFunction|GetNextAttackEffect) ; To telegraph
        )
        (:then_5
          (Variables|Default|SetTurnsBetweenAttack (Variables|/Game/Core/Blueprints/Enemies/PDA_EnemyData.PDA_EnemyData_C|GetTurnsBetweenAttack (Variables|Default|GetDataAsset)))
          (bind _aswui_enemy_healthbar (Utilities|Casting|CastToWUI_EnemyHealthbar (UserInterface|GetWidget (Variables|Default|GetWidget))))
          (Variables|/Game/Core/Blueprints/Enemies/WUI_EnemyHealthbar.WUI_EnemyHealthbar_C|SetTurnsBetweenAttack _aswui_enemy_healthbar (Variables|Default|GetTurnsBetweenAttack)))))
    (:else)))

(fn ProcessTurn
  (Utilities|FlowControl|Sequence
    (:then_0
      (if (== (Variables|Default|GetTurnCounter) (Variables|Default|GetTurnsBetweenAttack))
        (CallFunction|DoAttackEffect)
        (LocalVariables|SetbDidAttack true)
        (Variables|Default|SetTurnCounter 0)
        (CallFunction|GetNextAttackEffect)
        (else
          (Math|Integer|IncrementInt (Variables|Default|GetTurnCounter)))))
    (:then_1
      (bind _aswui_enemy_healthbar (Utilities|Casting|CastToWUI_EnemyHealthbar (UserInterface|GetWidget (Variables|Default|GetWidget))))
      (Variables|/Game/Core/Blueprints/Enemies/WUI_EnemyHealthbar.WUI_EnemyHealthbar_C|SetTurn%20Counter _aswui_enemy_healthbar (Variables|Default|GetTurnCounter))
      (return (LocalVariables|GetbDidAttack)))))

(fn DoAttackEffect
  (bind _trapcardaddamount (Variables|Default|GetTrapCardAddAmount))
  (bind _dataasset (Variables|Default|GetDataAsset))
  (bind _returnvalue (* _trapcardaddamount 4))
  (bind _bisboss (Variables|/Game/Core/Blueprints/Enemies/PDA_EnemyData.PDA_EnemyData_C|GetbIsBoss _dataasset))
  (bind _returnvalue_2 (Math|Integer|SelectInt _returnvalue _trapcardaddamount _bisboss))
  (Variables|Default|SetAttacking true) ; Could move later for others anims
  (switch Utilities|FlowControl|Switch|SwitchonE_EnemyAttackEffect (Variables|Default|GetNextAttackEffect)
    (:NewEnumerator2
      (bind _asbp_player_character (Utilities|Casting|CastToBP_PlayerCharacter (Game|GetPlayerCharacter 0)))
      (Default|TakeDamage _asbp_player_character (Variables|Default|GetDamage)))
    (:NewEnumerator3
      (if (>= (Variables|Default|GetTrapCardMax) (Variables|Default|GetTrapCardCounter))
        (bind _returnvalue_3 (Actor|GetActorOfClass "/Game/Core/Blueprints/Cards/BP_CardGrid.BP_CardGrid_C"))
        (bind _returnvalue_4 (Utilities|GetDataTableRow (Variables|/Game/Core/Blueprints/Cards/BP_CardGrid.BP_CardGrid_C|GetDataTable _returnvalue_3) "trap")
          (:then
            (Default|AddCardstoLevelLoopDeck _returnvalue_3 _returnvalue_4 _returnvalue_2)
            (Variables|Default|SetTrapCardCounter (+ (Variables|Default|GetTrapCardCounter) _returnvalue_2))))))))

(fn GetNextAttackEffect
  (bind _output_get (Variables|Default|SetNextAttackEffect (.OutItem (Utilities|Array|Random (Variables|Default|GetAttackEffects)))))
  (if (and (Utilities|Enum|Equal(Enum) _output_get "NewEnumerator3") (>= (Variables|Default|GetTrapCardCounter) (Variables|Default|GetTrapCardMax)))
    (Variables|Default|SetNextAttackEffect "NewEnumerator2"))
  (bind _aswui_enemy_healthbar (Utilities|Casting|CastToWUI_EnemyHealthbar (UserInterface|GetWidget (Variables|Default|GetWidget))))
  (Variables|/Game/Core/Blueprints/Enemies/WUI_EnemyHealthbar.WUI_EnemyHealthbar_C|SetNextEnemyAttackEffect _aswui_enemy_healthbar (Variables|Default|GetNextAttackEffect)))

(fn SetHitMaterialInstTextures
  (params (BaseMaterial :type Material%20Instance%20Dynamic%20Object%20Reference) (HitMaterial :type Material%20Instance%20Dynamic%20Object%20Reference))
  (for _array_element (Utilities|Array|MakeArray "Normal" "BaseColor" "Emissive" "OpacityMap" "AO/Roughness/Metallic")
    (bind _returnvalue (Rendering|Material|GetTextureParameterValue BaseMaterial _array_element :!class /Script/Engine.MaterialInstanceDynamic))
    (Rendering|Material|SetTextureParameterValue HitMaterial _array_element _returnvalue)))