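; Level map actor that generates each world's run of Battle, Shrine, Upgrade and Boss nodes and displays it in WUI_LevelMap.
; Node picks are random, constrained by counts, cooldowns and upgradeable cards, with a boss last.
; New maps cycle the world type, skipping the tutorial world after a new game and enabling freeplay on wrap.
; GM_Main events toggle the map, raise difficulty on wins and open Shrine or Upgrade screens.
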(event Custom|Create%20Map
  (params (bNewGame :type Boolean) (bLoading :type Boolean))
  ;[1 1 1] Comment
  (bind _wui_levelmap (Variables|Default|GetWUI_LevelMap) ; Remove old map if exists
    (:then
      (Widget|RemovefromParent _wui_levelmap)
      (Variables|Default|SetWUI_LevelMap 0)
      (Utilities|Platform|CollectGarbage))
    (:else
      _))
  (bind _returnvalue (UserInterface|CreateWidget "/Game/Core/Blueprints/GameMap/WUI_LevelMap.WUI_LevelMap_C" (Game|GetPlayerController 0) self)) ; Create new map
  (Variables|Default|SetWUI_LevelMap _returnvalue)
  (CallFunction|UpdateWorldTypeandIndex bNewGame bLoading)
  (bind _asgm_main (Utilities|Casting|CastToGM_Main (Game|GetGameMode)))
  (if bLoading
    _
    (else
      (CallFunction|GenerateLevelNodes)
      (Math|Integer|IncrementInt (Variables|/Game/Core/Blueprints/GM_Main.GM_Main_C|GetMapProgressions _asgm_main) ; For card grid, increment progressions
        (:%20%20
          _))))
  (Default|SetBackground (Variables|Default|GetWUI_LevelMap) (.Value (Utilities|Map|Find (Variables|Default|GetWorldTypeBackground) (Variables|/Game/Core/Blueprints/GM_Main.GM_Main_C|GetWorldType _asgm_main))))
  (Variables|/Game/Core/Blueprints/GameMap/WUI_LevelMap.WUI_LevelMap_C|SetNumNodes (Variables|Default|GetWUI_LevelMap) (Utilities|Array|Length (Variables|Default|GetLevel%20Nodes)))
  (for (_array_element _array_index) (Variables|Default|GetLevel%20Nodes) ; Create all map nodes
    (Default|AddNode (Variables|Default|GetWUI_LevelMap) _array_element (Utilities|Array|Get(acopy) (Variables|Default|GetLevel%20States) _array_index) _array_index))
  (if (not (UserInterface|Viewport|IsinViewport (Variables|Default|GetWUI_LevelMap))) ; Check if not in viewport
    (UserInterface|Viewport|AddtoViewport (Variables|Default|GetWUI_LevelMap) 0) ; Add to viewport
  )
  (Widget|SetVisibility (Variables|Default|GetWUI_LevelMap) "Hidden") ; Hide the map until needed
)

(event Custom|MapStart
  (params (bNewGame :type Boolean) (bLoading :type Boolean) (bPlayerWon :type Boolean))
  (bind _wui_speciallevel (Variables|Default|GetWUI_SpecialLevel)
    (:then
      (Widget|RemovefromParent _wui_speciallevel)
      (Variables|Default|SetWUI_SpecialLevel 0)
      (Utilities|Platform|CollectGarbage))
    (:else
      _))
  (Utilities|FlowControl|DelayUntilNextTick)
  (CallFunction|IncrementLevelDifficullty bPlayerWon)
  (Widget|SetVisibility (Variables|Default|GetWUI_LevelMap) "Visible"))

(event Custom|NextLevelStart
  (params (Difficulty :type Float%20%28double-precision%29) (LevelType :type E_LevelType%20Enum :default "NewEnumerator0") (bIsTutorial :type Boolean))
  (Widget|SetVisibility (Variables|Default|GetWUI_LevelMap) "Hidden"))

(event Custom|GenerateLevelNodes
  (Variables|Default|SetBattle%20Count 0) ; Reset counts
  (Variables|Default|SetShine%20Count 0)
  (Variables|Default|SetUpgrade%20Count 0)
  (bind _asgm_main (Utilities|Casting|CastToGM_Main (Game|GetGameMode)))
  (Utilities|Array|Clear (Variables|Default|GetLevel%20Nodes))
  (Utilities|Array|Clear (Variables|Default|GetLevel%20States))
  (for _index (range 0 (- (Math|Integer|SelectInt (Variables|Default|GetSmallerMapSize) (Variables|Default|GetBiggerMapSize) (Utilities|Enum|Equal(Enum) (Variables|/Game/Core/Blueprints/GM_Main.GM_Main_C|GetWorldType _asgm_main) "NewEnumerator3")) 1))
    (bind _output_get (Variables|Default|SetLevel%20Type (.OutItem (Utilities|Array|Random (select (Utilities|Enum|Equal(Enum) (Variables|/Game/Core/Blueprints/GM_Main.GM_Main_C|GetWorldType _asgm_main) "NewEnumerator3") (Utilities|Array|MakeArray "NewEnumerator0") (Utilities|Array|MakeArray "NewEnumerator0" "NewEnumerator1"))))))
    (CallFunction|AddLevelNode _output_get)
    (if (== _index 0)
      (Utilities|Array|Add (Variables|Default|GetLevel%20States) "NewEnumerator2")
      (else
        (Utilities|Array|Add (Variables|Default|GetLevel%20States) "NewEnumerator1"))))
  (CallFunction|AddBossNode)
  (Utilities|Array|Add (Variables|Default|GetLevel%20States) "NewEnumerator1"))

(event Custom|NextLevelPostStart
  (params (LevelType :type E_LevelType%20Enum :default "NewEnumerator0"))
  (switch Utilities|FlowControl|Switch|SwitchonE_LevelType LevelType
    (:NewEnumerator1
      (bind _returnvalue (UserInterface|CreateWidget "/Game/Core/Blueprints/GameMap/WUI_Shrine.WUI_Shrine_C"))
      (Variables|Default|SetWUI_SpecialLevel _returnvalue))
    (:NewEnumerator2
      (bind _returnvalue_2 (UserInterface|CreateWidget "/Game/Core/Blueprints/GameMap/WUI_Upgrade.WUI_Upgrade_C"))
      (Variables|Default|SetWUI_SpecialLevel _returnvalue_2)))
  (UserInterface|Viewport|AddtoViewport (Variables|Default|GetWUI_SpecialLevel) 0))

(event EventBeginPlay
  (bind _asgm_main (Utilities|Casting|CastToGM_Main (Game|GetGameMode)))
  (EventDispatchers|BindEventtoMapStart _asgm_main (delegate Custom|MapStart))
  (EventDispatchers|BindEventtoNextLevelStart _asgm_main (delegate Custom|NextLevelStart))
  (EventDispatchers|BindEventtoNextLevelPostStart _asgm_main (delegate Custom|NextLevelPostStart)))

(fn ConstructionScript)

(fn IncrementLevelDifficullty
  (params (Index :type Boolean))
  (bind _asgm_main (Utilities|Casting|CastToGM_Main (Game|GetGameMode)))
  (Variables|/Game/Core/Blueprints/GM_Main.GM_Main_C|SetDifficulty _asgm_main (+ (Variables|/Game/Core/Blueprints/GM_Main.GM_Main_C|GetDifficulty _asgm_main) (select Index (Variables|Default|GetDifficultyIncrementAmount) 0.0))))

(fn AddBossNode
  (Variables|Default|SetLevel%20Type "NewEnumerator4")
  (Utilities|Array|Add (Variables|Default|GetLevel%20Nodes) (Variables|Default|GetLevel%20Type)))

(fn AddLevelNode
  (params (Selection :type E_LevelType%20Enum :default "NewEnumerator0"))
  ;[1 1 1] Switch statment for type of nodes
  (switch Utilities|FlowControl|Switch|SwitchonE_LevelType Selection
    (:NewEnumerator0
      (if (<= (Variables|Default|GetBattle%20Count) 6)
        (Math|Integer|IncrementInt (Variables|Default|GetBattle%20Count)
          (:%20%20
            (Utilities|Array|Add (Variables|Default|GetLevel%20Nodes) (Variables|Default|GetLevel%20Type))))
        (elif (<= (Variables|Default|GetShine%20Count) 2)
          (Variables|Default|SetLevel%20Type "NewEnumerator1")
          (Utilities|Array|Add (Variables|Default|GetLevel%20Nodes) (Variables|Default|GetLevel%20Type))
          (Math|Integer|IncrementInt (Variables|Default|GetShine%20Count))
          (elif (<= (Variables|Default|GetUpgrade%20Count) 0)
            (LocalVariables|SetLPossibleUpgradeCount 0)
            (bind _returnvalue (Actor|GetActorOfClass "/Game/Core/Blueprints/Cards/BP_CardGrid.BP_CardGrid_C"))
            (bind _keys (Utilities|Map|Keys (Variables|/Game/Core/Blueprints/Cards/BP_CardGrid.BP_CardGrid_C|GetDeckDataInventory _returnvalue)))
            (for _array_element _keys
              (if (Utilities|Enum|NotEqual(Enum) (.CardType (Utilities|Struct|BreakST_CardData _array_element)) "NewEnumerator8")
                (bind _result (Math|Integer|IncrementInt (Math|Conversions|ToInteger(Byte) (.Value (Utilities|Map|Find (Variables|/Game/Core/Blueprints/Cards/BP_CardGrid.BP_CardGrid_C|GetDeckDataTier _returnvalue) _array_element))))
                  (:%20%20
                    (if (!= (Math|Integer|%(Integer) _result (|GetNumEnumEntries)) 0)
                      (Math|Integer|IncrementInt (LocalVariables|GetLPossibleUpgradeCount)))))))
            (Variables|Default|SetLevel%20Type (select (and (> (Variables|/Game/Core/Blueprints/GM_Main.GM_Main_C|GetMapProgressions (.AsGM%20Main (Utilities|Casting|CastToGM_Main (Game|GetGameMode)))) 1) (> (LocalVariables|GetLPossibleUpgradeCount) 0)) "NewEnumerator2" "NewEnumerator0")) ; Only start getting upgrades late-game
            (Utilities|Array|Add (Variables|Default|GetLevel%20Nodes) (Variables|Default|GetLevel%20Type))
            (Math|Integer|IncrementInt (Variables|Default|GetUpgrade%20Count))
            (else
              (Variables|Default|SetLevel%20Type "NewEnumerator0") ; Temp Upgrade Removal
              (Utilities|Array|Add (Variables|Default|GetLevel%20Nodes) (Variables|Default|GetLevel%20Type))
              (Math|Integer|DecrementInt (Variables|Default|GetUpgrade%20Countdown)
                (:%20%20
                  (Math|Integer|IncrementInt (Variables|Default|GetBattle%20Count)))))))))
    (:NewEnumerator1
      (if (and (<= (Variables|Default|GetShine%20Count) 2) (== (Variables|Default|GetShrine%20Countdown) 0))
        (Math|Integer|IncrementInt (Variables|Default|GetShine%20Count)
          (:%20%20
            (Utilities|Array|Add (Variables|Default|GetLevel%20Nodes) (Variables|Default|GetLevel%20Type))
            (Variables|Default|SetShrine%20Countdown 2)))
        (else
          (Variables|Default|SetLevel%20Type "NewEnumerator0")
          (Utilities|Array|Add (Variables|Default|GetLevel%20Nodes) (Variables|Default|GetLevel%20Type))
          (Math|Integer|DecrementInt (Variables|Default|GetShrine%20Countdown)
            (:%20%20
              (Math|Integer|IncrementInt (Variables|Default|GetBattle%20Count)))))))
    (:NewEnumerator2
      (if (and (<= (Variables|Default|GetUpgrade%20Count) 0) (== (Variables|Default|GetUpgrade%20Countdown) 0))
        ;;[1 1 1] Does not trigger
        (Math|Integer|IncrementInt (Variables|Default|GetUpgrade%20Count)
          (:%20%20
            (Utilities|Array|Add (Variables|Default|GetLevel%20Nodes) (Variables|Default|GetLevel%20Type))
            (Variables|Default|SetUpgrade%20Countdown 2)))
        (else
          (Variables|Default|SetLevel%20Type "NewEnumerator0")
          (Utilities|Array|Add (Variables|Default|GetLevel%20Nodes) (Variables|Default|GetLevel%20Type))
          (Math|Integer|DecrementInt (Variables|Default|GetUpgrade%20Countdown)
            (:%20%20
              (Math|Integer|IncrementInt (Variables|Default|GetBattle%20Count)))))))))

(fn UpdateWorldTypeandIndex
  (params (bNewGame :type Boolean) (bLoading :type Boolean))
  (if (not bLoading) ; Loading
    (if (not bNewGame) ; New Game
      (bind _result (Math|Integer|IncrementInt (Variables|Default|GetBackground%20Index))
        (:%20%20
          (if (== (Math|Integer|%(Integer) _result (|GetNumEnumEntries)) 0)
            (Variables|Default|SetBackground%20Index (Math|Integer|%(Integer) _result (|GetNumEnumEntries))) ; Wrap the index
            (bind _asgm_main (Utilities|Casting|CastToGM_Main (Game|GetGameMode)))
            (Variables|/Game/Core/Blueprints/GM_Main.GM_Main_C|SetbIsFreeplay _asgm_main true) ; Use alternate enemy pool in 'freeplay'
          )
          (if (Utilities|Enum|Equal(Enum) (Utilities|Enum|ByteToEnumE_WorldType (Math|Conversions|ToByte(Integer) (Variables|Default|GetBackground%20Index))) "NewEnumerator3") ; If Tutorial,
            (Math|Integer|IncrementInt (Variables|Default|GetBackground%20Index)
              (:%20%20
                _)))
          (bind _asgm_main_2 (Utilities|Casting|CastToGM_Main (Game|GetGameMode)))
          (Variables|/Game/Core/Blueprints/GM_Main.GM_Main_C|SetWorldType _asgm_main_2 (Utilities|Enum|ByteToEnumE_WorldType (Math|Conversions|ToByte(Integer) (Variables|Default|GetBackground%20Index)))) ; Update global world type
        ))
      (else
        (Variables|Default|SetBackground%20Index 0) ; Set to tutorial
        (bind _asgm_main_3 (Utilities|Casting|CastToGM_Main (Game|GetGameMode)))
        (Variables|/Game/Core/Blueprints/GM_Main.GM_Main_C|SetWorldType _asgm_main_3 (Utilities|Enum|ByteToEnumE_WorldType (Math|Conversions|ToByte(Integer) (Variables|Default|GetBackground%20Index)))) ; Update global world type
      ))
    (else
      (bind _asgm_main_4 (Utilities|Casting|CastToGM_Main (Game|GetGameMode)))
      (Variables|Default|SetBackground%20Index (Math|Conversions|ToInteger(Byte) (Variables|/Game/Core/Blueprints/GM_Main.GM_Main_C|GetWorldType _asgm_main_4))) ; Update Background Index
    )))