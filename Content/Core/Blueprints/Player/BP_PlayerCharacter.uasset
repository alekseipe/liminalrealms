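; Player character Blueprint that tracks health and stored block, refilling health and clearing block whenever GM_Main signals a new level.
; Incoming damage is absorbed by stored block first, then subtracted from health with a floor at zero, updating the WUI_PlayerHealthbar widget.
; Reaching zero health reports a failed level to GM_Main through LevelEnd.
; The next-turn event is bound but empty.
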(event Custom|NextTurn)

(event Custom|NextLevel
  (params (Difficulty :type Float%20%28double-precision%29))
  (Variables|Default|SetHealth (Variables|Default|GetMaxHealth))
  (CallFunction|UpdateHealthBar)
  (Variables|Default|SetStoredBlock 0.0))

(event EventBeginPlay
  (bind _asgm_main (Utilities|Casting|CastToGM_Main (Game|GetGameMode)))
  (EventDispatchers|BindEventtoNextLevel _asgm_main (delegate Custom|NextLevel))
  (EventDispatchers|BindEventtoNextTurn _asgm_main (delegate Custom|NextTurn)))

(fn ConstructionScript)

(fn UpdateHealthBar
  (bind _aswui_player_healthbar (Utilities|Casting|CastToWUI_PlayerHealthbar (UserInterface|GetWidget (Variables|Default|GetWidget))))
  (Default|SetHealthPercent _aswui_player_healthbar (Variables|Default|GetHealth) (Variables|Default|GetMaxHealth)))

(fn TakeDamage
  (params (Damage :type Float%20%28double-precision%29))
  (LocalVariables|SetLDamage Damage)
  (if (> (Variables|Default|GetHealth) 0.0) ; If alive
    (Utilities|ManageBlock
      (:OutputPin
        (LocalVariables|SetLDamageTaken (- (Variables|Default|GetHealth) (Math|Float|Max(Float) (- (Variables|Default|GetHealth) (LocalVariables|GetLDamage)) 0.0))) ; Gets damage taken (considering cutoff for minimum)
        (Variables|Default|SetHealth (Math|Float|Max(Float) (- (Variables|Default|GetHealth) (LocalVariables|GetLDamage)) 0.0))
        (CallFunction|UpdateHealthBar)
        (Development|PrintString (Utilities|String|ToString(Text) (Utilities|Text|FormatText "Player took {Damage} Damage!" (LocalVariables|GetLDamageTaken))))
        (if (<= (Variables|Default|GetHealth) 0.0)
          (CallFunction|EndLevel))))
    (else
      (return))))

(fn EndLevel
  (bind _asgm_main (Utilities|Casting|CastToGM_Main (Game|GetGameMode)))
  (Default|LevelEnd _asgm_main false))

(fn AddBlock
  (params (Block :type Float%20%28double-precision%29))
  (if (>= Block 0.0)
    (Variables|Default|SetStoredBlock (+ (Variables|Default|GetStoredBlock) Block))))